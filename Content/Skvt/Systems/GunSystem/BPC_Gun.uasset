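; BPC_Gun is a character component that equips a gun and handles switching in and out of aiming.
; On BeginPlay it caches the owning Character, spawns the configured gun class attached to a mesh socket, and saves the movement component's rotation rate.
; AimBegin and AimEnd toggle the aiming flag and swap rotation between following movement and following controller yaw, applying the aim rotation rate or restoring the saved one.
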(event Custom|AimBegin
  (bind _characterref (Variables|Default|GetCharacterRef))
  (bind _charactermovement (Variables|/Script/Engine.Character|GetCharacterMovement _characterref))
  (Variables|Default|SetIsAiming true)
  (Variables|/Script/Engine.CharacterMovementComponent|SetbOrientRotationToMovement _charactermovement false)
  (Variables|/Script/Engine.CharacterMovementComponent|SetbUseControllerDesiredRotation _charactermovement true)
  (Variables|/Script/Engine.CharacterMovementComponent|SetRotationRate _charactermovement (Variables|Default|GetAimRotationRate)))

(event Custom|AimEnd
  (bind _characterref (Variables|Default|GetCharacterRef))
  (bind _charactermovement (Variables|/Script/Engine.Character|GetCharacterMovement _characterref))
  (Variables|Default|SetIsAiming false)
  (Variables|/Script/Engine.CharacterMovementComponent|SetbOrientRotationToMovement _charactermovement true)
  (Variables|/Script/Engine.CharacterMovementComponent|SetbUseControllerDesiredRotation _charactermovement false)
  (Variables|/Script/Engine.CharacterMovementComponent|SetRotationRate (Variables|/Script/Engine.Character|GetCharacterMovement (Variables|Default|GetCharacterRef)) (Variables|Default|GetInitialRotationRate)))

(event EventBeginPlay
  (bind _ascharacter (Utilities|Casting|CastToCharacter (Components|GetOwner)))
  (Variables|Default|SetCharacterRef _ascharacter)
  (CallFunction|EquipGun)
  (Variables|Default|SetInitialRotationRate (Variables|/Script/Engine.CharacterMovementComponent|GetRotationRate (Variables|/Script/Engine.Character|GetCharacterMovement (Variables|Default|GetCharacterRef)))))

(fn EquipGun
  (bind _returnvalue (Game|SpawnActorfromClass (Variables|Default|GetGunClass) (Math|Transform|MakeTransform "0, 0, 0" "0, 0, 0" "1.000000,1.000000,1.000000") "Undefined" "MultiplyWithRoot" 0 0))
  (Transformation|AttachComponentToComponent _returnvalue (Variables|/Script/Engine.Character|GetMesh (Variables|Default|GetCharacterRef)) (Variables|Default|GetGunSocketName) "SnapToTarget" "SnapToTarget" "SnapToTarget" true))