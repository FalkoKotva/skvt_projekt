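; Actor component that makes its owner interactible by BP_SkvtBaseChar characters.
; Overlapping the owner's sphere or mesh (chosen by IsTrigger) sets it as the character's NearestInteractible, adds an overlay material and spawns floating text.
; End overlap clears all three.
; Interact branches by owner cast: wall sconces toggle and update their prompt, living NPCs lose movement and are deselected, generators fire an EMP explosion.
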(event Custom|ClearInteractible
  (params (OverlappedComponent :type Primitive%20Component%20Object%20Reference) (OtherActor :type Actor%20Object%20Reference) (OtherComp :type Primitive%20Component%20Object%20Reference) (OtherBodyIndex :type Integer))
  (bind _asbp_skvt_base_char (Utilities|Casting|CastToBP_SkvtBaseChar OtherActor))
  (CallFunction|Deselect)
  (Variables|/Game/Skvt/Characters/BP_SkvtBaseChar.BP_SkvtBaseChar_C|SetNearestInteractible _asbp_skvt_base_char 0))

(event Custom|SetNearestInteractible
  (params (OverlappedComponent :type Primitive%20Component%20Object%20Reference) (OtherActor :type Actor%20Object%20Reference) (OtherComp :type Primitive%20Component%20Object%20Reference) (OtherBodyIndex :type Integer) (bFromSweep :type Boolean) (SweepResult :type Hit%20Result%20Structure%20%28by%20ref%29))
  (bind _asbp_skvt_base_char (Utilities|Casting|CastToBP_SkvtBaseChar OtherActor))
  (Variables|/Game/Skvt/Characters/BP_SkvtBaseChar.BP_SkvtBaseChar_C|SetNearestInteractible _asbp_skvt_base_char self)
  (CallFunction|Select))

(event EventBeginPlay
  (bind _triggertooverlap (Variables|Components|GetTriggerToOverlap))
  (Variables|Default|SetMesh (Actor|GetComponentbyClass (Components|GetOwner) "/Script/Engine.MeshComponent"))
  (CallFunction|SetTrigger)
  (Utilities|FlowControl|Sequence
    (:then_0
      (Collision|BindEventtoOnComponentBeginOverlap _triggertooverlap (delegate Custom|SetNearestInteractible)))
    (:then_1
      (Collision|AssignOnComponentEndOverlap _triggertooverlap (delegate Custom|ClearInteractible)))))

(event EventSelect
  (bind _mesh (Variables|Default|GetMesh))
  (Rendering|Material|SetOverlayMaterial _mesh "/Game/Skvt/Assets/M_Overlay.M_Overlay" :!class /Script/Engine.MeshComponent)
  (bind _returnvalue (Game|SpawnActorfromClass "/Game/Skvt/UI/Textures/BP_InteractionText.BP_InteractionText_C" (Math|Conversions|ToTransform(Vector) (+ (Transformation|GetWorldLocation _mesh) "0.000000,0.000000,50.000000")) "AlwaysSpawn" "MultiplyWithRoot" 0 0))
  (Variables|Default|SetInteractionText _returnvalue)
  (CallFunction|SetInteractionText))

(event EventDeselect
  (Rendering|Material|SetOverlayMaterial (Variables|Default|GetMesh) 0 :!class /Script/Engine.MeshComponent)
  (Utilities|IsValid (Variables|Default|GetInteractionText)
    (:Is%20Valid
      (Actor|DestroyActor (Variables|Default|GetInteractionText))
      (Variables|Default|SetInteractionText 0))))

(event EventInteract
  (bind _returnvalue (Components|GetOwner))
  (Utilities|FlowControl|Sequence
    (:then_0
      (bind _asbp_wall_sconce (Utilities|Casting|CastToBP_WallSconce _returnvalue))
      (Default|ToggleonInternal _asbp_wall_sconce (not (Variables|/Game/Skvt/Blueprints/Light/BP_WallSconce.BP_WallSconce_C|GetIsOn _asbp_wall_sconce)))
      (if (not (Variables|/Game/Skvt/Blueprints/Light/BP_WallSconce.BP_WallSconce_C|GetIsOn _asbp_wall_sconce))
        (Variables|Config|SetInteractionTextText "Switch On")
        (CallFunction|SetInteractionText)
        (else
          (Variables|Config|SetInteractionTextText "Switch Off")
          (CallFunction|SetInteractionText))))
    (:then_1
      (bind _asbp_npc_base (Utilities|Casting|CastToBP_NPC_base _returnvalue))
      (if (not (Default|IsDead (Variables|/Game/Skvt/Characters/NPC/BP_NPC_base.BP_NPC_base_C|GetSkvtHealth _asbp_npc_base)))
        (Pawn|Components|CharacterMovement|DisableMovement (Variables|/Script/Engine.Character|GetCharacterMovement _asbp_npc_base))
        (CallFunction|Deselect)))
    (:then_2
      (bind _asbp_generator (Utilities|Casting|CastToBP_Generator _returnvalue))
      (Default|ActivateEmpExplosion (Variables|/Game/Skvt/Blueprints/Explosion/BP_Generator.BP_Generator_C|GetBPC_EMP_Explosion _asbp_generator)))))

(event EventSetInteractionText
  (bind _interactiontext (Variables|Default|GetInteractionText))
  (Utilities|IsValid _interactiontext
    (:Is%20Valid
      (Rendering|Components|TextRender|SetText (Variables|/Script/Engine.TextRenderActor|GetTextRender _interactiontext) (Variables|Config|GetInteractionTextText)))))

(fn SetTrigger
  (if (Variables|Config|GetIsTrigger)
    (Variables|Components|SetTriggerToOverlap (Actor|GetComponentbyClass (Components|GetOwner) "/Script/Engine.SphereComponent"))
    (else
      (Variables|Components|SetTriggerToOverlap (Variables|Default|GetMesh)))))