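; Base NPC character Blueprint that can take damage, attack, die and jump to a target point.
; Damage and attacks are delegated to the SkvtHealth component, with a hit montage played on any damage.
; On the component's death event the mesh switches to physics simulation, movement is disabled and the actor is destroyed after a delay.
; JumpToDestination launches the character along a suggested projectile arc to a point raised above the destination.
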(event OnCharacterDeath(SkvtHealth)
  (Physics|SetSimulatePhysics (Variables|Character|GetMesh) true)
  (Pawn|Components|CharacterMovement|DisableMovement (Variables|Character|GetCharacterMovement))
  (Utilities|Time|SetTimerbyEvent (delegate Custom|Destroy) 6.0))

(event Custom|JumpToDestination
  (params (Destination :type Vector))
  (bind (_x _y _z) (Math|Vector|BreakVector Destination))
  (bind _outlaunchvelocity (Game|SuggestProjectileVelocityCustomArc (Transformation|GetActorLocation) (Math|Vector|MakeVector _x _y (+ _z 175.0)) 0.0 0.5))
  (Character|LaunchCharacter _outlaunchvelocity true true))

(event Custom|Attack
  (Default|Attack (Variables|Default|GetSkvtHealth) (Variables|Default|GetAttackStart) (Variables|Default|GetAttackEnd)))

(event Custom|Destroy
  (Actor|DestroyActor))

(event EventBeginPlay)

(event Collision|EventActorBeginOverlap
  (params (OtherActor :type Actor%20Object%20Reference)))

(event EventTick
  (params (DeltaSeconds :type Float%20%28single-precision%29)))

(event Game|Damage|EventAnyDamage
  (params (Damage :type Float%20%28single-precision%29) (DamageType :type Damage%20Type%20Object%20Reference) (InstigatedBy :type Controller%20Object%20Reference) (DamageCauser :type Actor%20Object%20Reference))
  (Default|ProcessDamage (Variables|Default|GetSkvtHealth) Damage)
  (Animation|PlayAnimMontage "/Game/Skvt/Characters/Animations/Attacks/AM_Hit_punch.AM_Hit_punch" 1.0 "None"))

(fn ConstructionScript)