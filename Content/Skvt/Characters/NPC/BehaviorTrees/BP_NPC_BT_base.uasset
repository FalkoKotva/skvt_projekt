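; Base NPC character for behavior-tree AI that spots the player, takes damage and dies.
; On possession it caches its AIC_BT_NPCBase controller; when PawnSensing sees the player, it notifies that controller and raises walk speed.
; Damage goes to the SkvtHealth component and plays a hit montage.
; The component's death event disables mesh physics and movement, then a timer destroys the actor after a short delay.
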(event OnSeePawn(PawnSensing)
  (params (Pawn :type Pawn%20Object%20Reference))
  (if (== Pawn (Game|GetPlayerCharacter 0))
    (Default|SeenPlayer (Variables|Default|GetControllerRef) Pawn)
    (Variables|/Script/Engine.CharacterMovementComponent|SetMaxWalkSpeed (Variables|Character|GetCharacterMovement) 6e+02)))

(event OnCharacterDeath(SkvtHealth)
  (CallFunction|TriggerCharacterDeath))

(event EventBeginPlay
  (|CallParentFunction) ; This node is disabled and will not be called.\nDrag off pins to build functionality.
)

(event Collision|EventActorBeginOverlap
  (params (OtherActor :type Actor%20Object%20Reference))
  (|CallParentFunction OtherActor) ; This node is disabled and will not be called.\nDrag off pins to build functionality.
)

(event EventTick
  (params (DeltaSeconds :type Float%20%28single-precision%29))
  (|CallParentFunction DeltaSeconds) ; This node is disabled and will not be called.\nDrag off pins to build functionality.
)

(event EventPossessed
  (params (NewController :type Controller%20Object%20Reference))
  (bind _asaic_bt_npcbase (Utilities|Casting|CastToAIC_BT_NPCBase NewController))
  (Variables|Default|SetControllerRef _asaic_bt_npcbase))

(event Game|Damage|EventAnyDamage
  (params (Damage :type Float%20%28single-precision%29) (DamageType :type Damage%20Type%20Object%20Reference) (InstigatedBy :type Controller%20Object%20Reference) (DamageCauser :type Actor%20Object%20Reference))
  (Default|ProcessDamage (Variables|Default|GetSkvtHealth) Damage)
  (Animation|PlayAnimMontage "/Game/Skvt/Characters/Animations/Attacks/AM_Hit_punch.AM_Hit_punch" 1.0 "None"))

(fn ConstructionScript
  (|CallParentFunction))

(fn TriggerCharacterDeath
  (Physics|SetSimulatePhysics (Variables|Character|GetMesh) false)
  (Pawn|Components|CharacterMovement|DisableMovement (Variables|Character|GetCharacterMovement))
  (Utilities|Time|SetTimerbyFunctionName 0 "FinishCharacterDeath" 3.0))

(fn FinishCharacterDeath
  (Actor|DestroyActor))