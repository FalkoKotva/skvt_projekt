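; Actor component that gives its owner an EMP explosion, disabling nearby wall sconces and screens.
; On BeginPlay it adds a collision sphere of configurable radius to the owner.
; ActivateEmpExplosion spawns the particle effect and sound, then passes the sphere's overlapping actors to the EMP event.
; Tagged, undestroyed sconces get sparks, switch off and are marked destroyed, while screens have their webpage hidden.
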(event Custom|OnEmpExplosion_Event
  (params (OverlapingActors :type Array%20of%20Object%20Object%20References))
  (for _array_element OverlapingActors
    (bind _asactor (Utilities|Casting|CastToActor _array_element))
    (Utilities|FlowControl|Sequence
      (:then_0
        ;[1 1 1] Add Sparks effect to Emped actors BP_WallSconce with tag PossibleEmp
        (bind _asbp_wall_sconce (Utilities|Casting|CastToBP_WallSconce _asactor))
        (if (and (not (Variables|/Game/Skvt/Blueprints/Light/BP_WallSconce.BP_WallSconce_C|GetIsDestroyed _asbp_wall_sconce)) (Actor|ActorHasTag _asactor (Variables|Default|GetPossibleEmpTag)))
          (bind _returnvalue (Game|AddComponentbyClass _asactor "/Script/Engine.ParticleSystemComponent" false))
          (Effects|Components|ParticleSystem|SetTemplate _returnvalue "/Game/StarterContent/Particles/P_Sparks.P_Sparks")
          (Default|ToggleonInternal _asbp_wall_sconce false)
          (Variables|/Game/Skvt/Blueprints/Light/BP_WallSconce.BP_WallSconce_C|SetIsDestroyed _asbp_wall_sconce true)))
      (:then_1
        (bind _asbp_skvt_screen (Utilities|Casting|CastToBP_SkvtScreen _asactor))
        (Rendering|SetVisibility (Variables|/Game/Skvt/Blueprints/Screen/BP_SkvtScreen.BP_SkvtScreen_C|GetWebpage _asbp_skvt_screen) false false)))))

(event EventTick
  (params (DeltaSeconds :type Float%20%28single-precision%29)))

(event EventBeginPlay
  (bind _returnvalue (Components|GetOwner))
  (Utilities|IsValid _returnvalue
    (:Is%20Valid
      (bind _returnvalue_2 (Game|AddComponentbyClass _returnvalue "/Script/Engine.SphereComponent" false))
      (Components|Sphere|SetSphereRadius _returnvalue_2 (Variables|Default|GetRadiusSize) true)
      (Variables|Default|SetCollisionRadiusRef _returnvalue_2))))

(fn GetOverlapingActors
  (bind _collisionradiusref (Variables|Default|GetCollisionRadiusRef))
  (bind _overlappingactors (Collision|GetOverlappingActors _collisionradiusref "/Script/Engine.Actor" :!class /Script/Engine.PrimitiveComponent))
  (Utilities|IsValid _collisionradiusref
    (:Is%20Valid
      (if (Utilities|Array|IsNotEmpty _overlappingactors)
        (CallFunction|OnEmpExplosionEvent _overlappingactors)))))

(fn ActivateEmpExplosion
  (bind _returnvalue (Components|GetOwner))
  ;[1 1 1] Add particle effect + sound of EMP explosion
  (bind _returnvalue_2 (Game|AddComponentbyClass _returnvalue "/Script/Engine.ParticleSystemComponent" false))
  (Effects|Components|ParticleSystem|SetTemplate _returnvalue_2 "/Game/EMP_Explosion.EMP_Explosion")
  (Audio|PlaySoundatLocation "/Game/StarterContent/Audio/Explosion01.Explosion01" (Transformation|GetActorLocation _returnvalue) "0, 0, 0" 1.0 1.0 0.0 0 0 0 0)
  (CallFunction|GetOverlapingActors))