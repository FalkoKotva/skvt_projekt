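; BP_Platform is a platform that lights its lamps while overlapped and fires an EMP blast after it is left.
; Box overlap begin and end switch every entry in the Lamps array on or off through ToggleLights, with no filter on the overlapping actor.
; End overlap also starts a one-second timer that activates the BPCEMPExplosion component.
; Tick draws a debug sphere at the platform showing the EMP radius.
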(event OnComponentBeginOverlap(Box)
  (params (OverlappedComponent :type Primitive%20Component%20Object%20Reference) (OtherActor :type Actor%20Object%20Reference) (OtherComp :type Primitive%20Component%20Object%20Reference) (OtherBodyIndex :type Integer) (bFromSweep :type Boolean) (SweepResult :type Hit%20Result%20Structure%20%28by%20ref%29))
  (CallFunction|ToggleLights true))

(event OnComponentEndOverlap(Box)
  (params (OverlappedComponent :type Primitive%20Component%20Object%20Reference) (OtherActor :type Actor%20Object%20Reference) (OtherComp :type Primitive%20Component%20Object%20Reference) (OtherBodyIndex :type Integer))
  (CallFunction|ToggleLights false)
  (Utilities|Time|SetTimerbyEvent (delegate Custom|EMP_Explosion) 1.0))

(event Custom|EMP_Explosion
  (Default|ActivateEmpExplosion (Variables|Default|GetBPC_EMP_Explosion)))

(event EventBeginPlay)

(event EventTick
  (params (DeltaSeconds :type Float%20%28single-precision%29))
  (Rendering|Debug|DrawDebugSphere (Transformation|GetWorldLocation (Variables|Default|GetPlatform)) (Variables|/Game/Skvt/Blueprints/Explosion/BPC_EMP_Explosion.BPC_EMP_Explosion_C|GetRadiusSize (Variables|Default|GetBPC_EMP_Explosion)) 24 "(R=0.358127,G=0.483407,B=1.000000,A=1.000000)" 0.0 1.0))

(fn ConstructionScript)

(fn ToggleLights
  (params (IsOn :type Boolean))
  (for _array_element (Variables|Default|GetLamps)
    (Default|ToggleonInternal _array_element IsOn)))