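; Trigger platform that drives a set of linked Electronics objects when actors step on or off it.
; On any actor overlap it tells each entry in the Electronics array to change color, then switches them all on.
; When an overlap ends it switches them all off, with no filtering or counting of overlapping actors.
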(event Custom|ChangeColor
  (for _array_element (Variables|Default|GetElectronics)
    (Default|ChangeColorInternal _array_element)))

(event EventBeginPlay)

(event EventTick
  (params (DeltaSeconds :type Float%20%28single-precision%29)))

(event Collision|EventActorBeginOverlap
  (params (OtherActor :type Actor%20Object%20Reference))
  (CallFunction|ChangeColor)
  (CallFunction|Toggleon true))

(event Collision|EventActorEndOverlap
  (params (OtherActor :type Actor%20Object%20Reference))
  (CallFunction|Toggleon false))

(fn ConstructionScript)

(fn Toggleon
  (params (IsOn :type Boolean))
  (for _array_element (Variables|Default|GetElectronics)
    (Default|ToggleonInternal _array_element IsOn)))